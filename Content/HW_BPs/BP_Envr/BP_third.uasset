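; BP_third is an environment Blueprint whose cube changes look when a BP_BALL actor overlaps it.
; On overlap, it casts the other actor to BP_BALL and, through a DoOnce, swaps the Cube's first material to FlowMaps a single time.
; It then calls the parent overlap handler, while BeginPlay, Tick and the construction script add no logic of their own.
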(event EventBeginPlay
  (|CallParentFunction) ; This node is disabled and will not be called.\nDrag off pins to build functionality.
)

(event Collision|EventActorBeginOverlap
  (params (OtherActor :type Actor%20Object%20Reference))
  (Utilities|Casting|CastToBP_BALL OtherActor)
  (Utilities|FlowControl|Sequence
    (:then_0
      (Utilities|FlowControl|DoOnce false
        (:Completed
          (Rendering|Material|SetMaterial (Variables|Default|GetCube) 0 "/Engine/Functions/Engine_MaterialFunctions02/ExampleContent/FlowMaps.FlowMaps"))))
    (:then_1
      (|CallParentFunction OtherActor))))

(event EventTick
  (params (DeltaSeconds :type Float%20%28single-precision%29))
  (|CallParentFunction DeltaSeconds) ; This node is disabled and will not be called.\nDrag off pins to build functionality.
)

(fn ConstructionScript
  (|CallParentFunction))