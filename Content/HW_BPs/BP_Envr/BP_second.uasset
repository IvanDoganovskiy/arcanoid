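; BP_second is an environment actor whose cube shrinks each time a BP_BALL overlaps it.
; BeginPlay stores five percent of the cube's starting world scale as a fixed step.
; Each ball overlap subtracts that step until the scale is within tolerance of the step size, then passes the event to the parent class.
; Other actors are ignored, and Tick is disabled.
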(event EventBeginPlay
  (|CallParentFunction)
  (bind _output_get (Variables|Default|SetDelta%20Scale (* (Transformation|GetWorldScale (Variables|Default|GetCube)) 0.05))))

(event Collision|EventActorBeginOverlap
  (params (OtherActor :type Actor%20Object%20Reference))
  (Utilities|Casting|CastToBP_BALL OtherActor)
  (if (Math|Vector|NotEqual(Vector) (stale EventBeginPlay _output_get) (Transformation|GetWorldScale (Variables|Default|GetCube)) 0.1)
    (Transformation|SetWorldScale3D (Variables|Default|GetCube) (- (Transformation|GetWorldScale (Variables|Default|GetCube)) (Variables|Default|GetDelta%20Scale))))
  (|CallParentFunction OtherActor))

(event EventTick
  (params (DeltaSeconds :type Float%20%28single-precision%29))
  (|CallParentFunction DeltaSeconds) ; This node is disabled and will not be called.\nDrag off pins to build functionality.
)

(fn ConstructionScript
  (|CallParentFunction))